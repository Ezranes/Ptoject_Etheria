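; Gameplay game mode that spawns player characters into the level.
; On BeginPlay it caches a reference to the MainGameInstance.
; Its SpawnCharacter event spawns the given character class at a randomly chosen PlayerStart and has the supplied controller possess it.
; The random pick does not check whether that start is already occupied.
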(event `self.ReceiveBeginPlay`
  (bind _asmain_game_instance (cast `/Game/_Game/_Core/Framework/General/MainGameInstance` (`GameplayStatics.GetGameInstance`)))
  (set `self.As Maingame Instance` _asmain_game_instance))

(event `SpawnCharacter`
  (params (Character :type "Character Class Reference") (controller :type "Controller Object Reference"))
  ;[1 1 1] Spawn Character
  (bind _outactors (`GameplayStatics.GetAllActorsOfClass` "/Script/Engine.PlayerStart"))
  (bind _returnvalue (`|SpawnActorFromClass` Character (`self.GetTransform` (`|GetArrayItem` _outactors (`KismetMathLibrary.RandomIntegerInRange` 0 (- (`KismetArrayLibrary.Array_Length` _outactors) 1)))) "Undefined" "OverrideRootScale" null null))
  (`Controller.Possess` controller _returnvalue))

(fn `UserConstructionScript`)