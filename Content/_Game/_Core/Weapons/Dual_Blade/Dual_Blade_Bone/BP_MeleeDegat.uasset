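; BP_MeleeDegat is a short-lived melee damage hitbox for the Dual Blade Bone weapon.
; When its box begins overlapping a _Mother actor, it applies a fixed amount of damage, prints a debug message and destroys itself.
; Any other overlap also destroys it, after a brief delay if that actor is the owner.
; The server and multicast damage events are empty stubs.
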(event `self.Box.OnComponentBeginOverlap`
  (params (OverlappedComponent :type "PrimitiveComponent Object Reference") (OtherActor :type "Actor Object Reference") (OtherComp :type "PrimitiveComponent Object Reference") (OtherBodyIndex :type Integer) (bFromSweep :type Boolean) (SweepResult :type "HitResult Structure (by ref)"))
  (bind _as_mother (cast `/Game/_Game/_Core/IA/_Mother` OtherActor)
    (:`then`
      (`GameplayStatics.ApplyDamage` _as_mother 20.0 null self)
      (`KismetSystemLibrary.PrintString` "-20")
      (`self.K2_DestroyActor`))
    (:`CastFailed`
      (if (!= OtherActor (`self.GetOwner`))
        (`self.K2_DestroyActor`)
        (else
          (`KismetSystemLibrary.Delay` 0.1)
          (`self.K2_DestroyActor`))))))

(event `SRV_Apply_Damage`)

(event `MC_Aply_Damage`)

(fn `UserConstructionScript`)