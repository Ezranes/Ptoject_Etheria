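; PC_Lobby is the lobby player controller, which shows the lobby UI and passes player list updates to it.
; On BeginPlay it caches the MainGameInstance and, if that cast succeeds and the controller is local, creates WBP_Lobby and adds it to the viewport.
; The UpdatePlayerList event forwards the received list to the widget's UpdateListPlayers.
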(event `self.ReceiveBeginPlay`
  (`|ExecutionSequence`
    (:`then_0`
      (bind _asmain_game_instance (cast `/Game/_Game/_Core/Framework/General/MainGameInstance` (`GameplayStatics.GetGameInstance`)))
      (set `self.GameInstance` _asmain_game_instance))
    (:`then_1`
      (if (`self.IsLocalPlayerController`)
        (`|ExecutionSequence`
          (:`then_0`
            (bind _returnvalue (`|CreateWidget` "/Game/_Game/UI/MainMenu/Pages/WBP_Lobby.WBP_Lobby_C" self))
            (bind _output_get (set `self.WBPLobby` _returnvalue))
            (`UserWidget.AddToViewport` _output_get 0)))))))

(event `UpdatePlayerList`
  (params (PlayerList :type "Array of /Game/_Game/_Core/Player/Lobby/PC_Lobby Object Reference"))
  (`/Game/_Game/UI/MainMenu/Pages/WBP_Lobby.UpdateListPlayers` (`self.WBPLobby`) PlayerList))

(fn `UserConstructionScript`)