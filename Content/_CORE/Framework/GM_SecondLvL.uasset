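; GM_SecondLvL is a game mode, apparently for the second level, that spawns and possesses player characters.
; Two custom events, one named for Smelfaria and one for Blingiskan, each take a class and a target controller.
; Each picks a random PlayerStart, spawns the given class at its transform and has the controller possess the result.
; The two events have identical logic, and the supplied class determines what spawns.
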(event `Spawn Actors melfaria`
  (params (Class :type "Character Class Reference") (Target :type "Controller Object Reference"))
  (bind _outactors (`GameplayStatics.GetAllActorsOfClass` "/Script/Engine.PlayerStart"))
  (bind _returnvalue (`|SpawnActorFromClass` Class (`self.GetTransform` (`|GetArrayItem` _outactors (`KismetMathLibrary.RandomIntegerInRange` 0 (- (`KismetArrayLibrary.Array_Length` _outactors) 1)))) "Undefined" "OverrideRootScale" null null))
  (`Controller.Possess` Target _returnvalue))

(event `Spawn character Blingiskan`
  (params (`Class 2` :type "Character Class Reference") (Target2 :type "Controller Object Reference"))
  (bind _outactors (`GameplayStatics.GetAllActorsOfClass` "/Script/Engine.PlayerStart"))
  (bind _returnvalue (`|SpawnActorFromClass` `Class 2` (`self.GetTransform` (`|GetArrayItem` _outactors (`KismetMathLibrary.RandomIntegerInRange` 0 (- (`KismetArrayLibrary.Array_Length` _outactors) 1)))) "Undefined" "OverrideRootScale" null null))
  (`Controller.Possess` Target2 _returnvalue))

(fn `UserConstructionScript`)