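; PC_Menu is the main menu player controller that shows the menu and relays session requests.
; On BeginPlay it creates WBP_Mainmenus, adds it to the viewport and caches the MaingameInstance.
; Its create and join events fetch player controller 0 as PC_Menu and call CreateSession or FindSession on that game instance.
; Both events pass along the Blingiskan and Melfaria selection flags.
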(event `self.ReceiveBeginPlay`
  (`|ExecutionSequence`
    (:`then_0`
      (bind _returnvalue (`|CreateWidget` "/Game/UI/Main_menu/WBP_Mainmenus.WBP_Mainmenus_C"))
      (`UserWidget.AddToViewport` _returnvalue 0)
      (set `self.WBP Main Menus` _returnvalue))
    (:`then_1`
      (bind _asmaingame_instance (cast `/Game/_CORE/Framework/MaingameInstance` (`GameplayStatics.GetGameInstance`)))
      (set `self.maingameinstance` _asmaingame_instance))))

(event `CreateSessiongame`
  (params (`Selected is Blingiskan` :type Boolean) (`Selected Is Melfaria` :type Boolean))
  (bind _aspc_menu (cast `/Game/_CORE/Player/player_controller/Main_menus/PC_Menu` (`GameplayStatics.GetPlayerController` 0)))
  (`/Game/_CORE/Framework/MaingameInstance.Create Session` (`/Game/_CORE/Player/player_controller/Main_menus/PC_Menu.maingameinstance` _aspc_menu) `Selected is Blingiskan` `Selected Is Melfaria`))

(event `JoinSessionGame`
  (params (`Selected is blingiskan` :type Boolean) (`selected is Melfaria` :type Boolean))
  (bind _aspc_menu (cast `/Game/_CORE/Player/player_controller/Main_menus/PC_Menu` (`GameplayStatics.GetPlayerController` 0)))
  (`/Game/_CORE/Framework/MaingameInstance.Find session` (`/Game/_CORE/Player/player_controller/Main_menus/PC_Menu.maingameinstance` _aspc_menu) `Selected is blingiskan` `selected is Melfaria`))

(fn `UserConstructionScript`)