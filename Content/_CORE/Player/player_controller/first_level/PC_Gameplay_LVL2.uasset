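; PC_Gameplay_LVL2 is the player controller for the second gameplay level, setting up the HUD and requesting player character spawns.
; On BeginPlay it creates the main gameplay widget, adds it to the viewport and caches the game instance.
; Two custom events ask GM_Gameplay to spawn either the Ethereal character (Melfaria) or the Physical character (Blingiskan), passing player controller 0 as the target.
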(event `self.ReceiveBeginPlay`
  (`|ExecutionSequence`
    (:`then_0`
      (bind _returnvalue (`|CreateWidget` "/Game/UI/MainGame/Pages/WBP_MainGameplay.WBP_MainGameplay_C"))
      (`UserWidget.AddToViewport` _returnvalue 0)
      (set `self.WBP_MainGamePlay` _returnvalue))
    (:`then_1`
      (bind _asmaingame_instance (cast `/Game/_CORE/Framework/MaingameInstance` (`GameplayStatics.GetGameInstance`)))
      (set `self.As Maingame Instance` _asmaingame_instance))))

(event `melfaria spawning call`
  (bind _asgm_gameplay (cast `/Game/_CORE/Framework/GM_Gameplay` (`GameplayStatics.GetGameMode`)))
  (bind _output_get (set `self.As GM Gameplay` _asgm_gameplay))
  (`/Game/_CORE/Framework/GM_Gameplay.Spawn Actors melfaria` _output_get "/Game/_CORE/Player/characters/Bp_Ethereal_Character.Bp_Ethereal_Character_C" (`GameplayStatics.GetPlayerController` 0)))

(event `Blingiskan spawning call`
  (bind _asgm_gameplay (cast `/Game/_CORE/Framework/GM_Gameplay` (`GameplayStatics.GetGameMode`)))
  (bind _output_get (set `self.As GM Gameplay` _asgm_gameplay))
  (`/Game/_CORE/Framework/GM_Gameplay.Spawn character Blingiskan` _output_get "/Game/_CORE/Player/characters/BP_Physical_Character.BP_Physical_Character_C" (`GameplayStatics.GetPlayerController` 0)))

(fn `UserConstructionScript`)