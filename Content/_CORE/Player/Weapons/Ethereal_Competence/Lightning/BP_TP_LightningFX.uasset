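; Chain-lightning FX actor that hops between nearby Dummyxtarget actors, drawing an electric arc along the chain.
; Sphere overlaps maintain the in-range candidates, skipping targets already recorded as touched on entry.
; Each Tick it teleports to the nearest candidate, marks it touched, then points the ElectricArcs beam parameters from there to the next nearest, raised above actor origins.
; It destroys itself when no candidate remains.
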(event `self.ReceiveTick`
  (params (DeltaSeconds :type "Float (single-precision)"))
  (bind _dummyinrange (`self.DummyInRange`))
  (bind _electric_arcs (`self.electric_arcs`))
  (bind (_returnvalue_x _returnvalue_y _returnvalue_z) (`KismetMathLibrary.BreakVector` (`self.K2_GetActorLocation` self)))
  ;[1 1 1] Logique de déplacement de l'actor
  (bind _actor_return (`/Game/_CORE/Library/FLBP_actors.Get Nearest Actors` (`self.Sphere`) (`self.DummyInRange`) self))
  (`/Engine/EditorBlueprintResources/StandardMacros.IsValid` _actor_return
    (:`Is Valid`
      (bind _output_get (set `self.Actor Return` _actor_return))
      (`KismetArrayLibrary.Array_AddUnique` (`self.ActorAlreadyTouched`) _output_get)
      (`self.K2_SetActorLocation` (`self.K2_GetActorLocation` (`self.Actor Return`)))
      (`KismetArrayLibrary.Array_RemoveItem` _dummyinrange (`self.Actor Return`))
      (bind _actor_return_2 (`/Game/_CORE/Library/FLBP_actors.Get Nearest Actors` (`self.Sphere`) _dummyinrange self))
      (`/Engine/EditorBlueprintResources/StandardMacros.IsValid` _actor_return_2
        (:`Is Valid`
          (`FXSystemComponent.SetVectorParameter` _electric_arcs "User.BeamStart" (`KismetMathLibrary.MakeVector` _returnvalue_x _returnvalue_y (+ _returnvalue_z 100.0)))
          (bind (_returnvalue_x_2 _returnvalue_y_2 _returnvalue_z_2) (`KismetMathLibrary.BreakVector` (`self.K2_GetActorLocation` _actor_return_2)))
          (`FXSystemComponent.SetVectorParameter` _electric_arcs "User.BeamEnd" (`KismetMathLibrary.MakeVector` _returnvalue_x_2 _returnvalue_y_2 (+ _returnvalue_z_2 100.0))))))
    (:`Is Not Valid`
      (`self.K2_DestroyActor`))))

(event `self.Sphere.OnComponentBeginOverlap`
  (params (OverlappedComponent :type "PrimitiveComponent Object Reference") (OtherActor :type "Actor Object Reference") (OtherComp :type "PrimitiveComponent Object Reference") (OtherBodyIndex :type Integer) (bFromSweep :type Boolean) (SweepResult :type "HitResult Structure (by ref)"))
  ;[1 1 1] Logique de cast
  (bind _asdummyxtarget (cast `/Game/_CORE/Player/Props/Dummyxtarget` OtherActor))
  (if (== (`KismetArrayLibrary.Array_Find` (`self.ActorAlreadyTouched`) _asdummyxtarget) -1)
    (`KismetArrayLibrary.Array_AddUnique` (`self.DummyInRange`) _asdummyxtarget)))

(event `self.Sphere.OnComponentEndOverlap`
  (params (OverlappedComponent :type "PrimitiveComponent Object Reference") (OtherActor :type "Actor Object Reference") (OtherComp :type "PrimitiveComponent Object Reference") (OtherBodyIndex :type Integer))
  ;[1 1 1] Logique de cast
  (bind _asdummyxtarget (cast `/Game/_CORE/Player/Props/Dummyxtarget` OtherActor))
  (`KismetArrayLibrary.Array_RemoveItem` (`self.DummyInRange`) _asdummyxtarget))

(fn `UserConstructionScript`)