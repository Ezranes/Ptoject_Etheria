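; Playable first-person physical character with a sword attack and three skills: Rush, dagger throw and Débarquement.
; Fire, A and E spawn melee damage, dagger and crush actors, with delayed cooldowns only on melee and dagger.
; R line-traces forward from the camera, then teleports with sweep if a downward trace finds ground.
; Each action has a busy flag, though Rush and Débarquement clear theirs immediately.
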(event `InputAction|Fire`
  (params (Key :type "Key Structure"))
  ;[1 1 1] Coup d'épée
  (:`Pressed`
    (`self.Attack server`)))

(event `Attack server`
  (bind _spawnmeleedegat (`self.SpawnMeleeDegat`))
  ;[1 1 1] Coup d'épée
  (if (not (`self.Attacking`))
    (set `self.Attacking` true)
    (`|SpawnActorFromClass` "/Game/_Game/_Core/Weapons/Dual_Blade/Dual_Blade_Bone/BP_MeleeDegat.BP_MeleeDegat_C" (`KismetMathLibrary.MakeTransform` (`SceneComponent.K2_GetComponentLocation` _spawnmeleedegat) (`SceneComponent.K2_GetComponentRotation` _spawnmeleedegat)) "Undefined" "OverrideRootScale" self null)
    (`KismetSystemLibrary.Delay` 0.2)
    (set `self.Attacking` false)))

(event `Key|R`
  (params (Key :type "Key Structure"))
  ;[1 1 1] Rush
  (:`Pressed`
    (`self.Rush`)))

(event `Rush`
  (bind _firstpersoncamera (`self.FirstPersonCamera`))
  (bind _returnvalue (`SceneComponent.K2_GetComponentLocation` (`self.FirstPersonCamera`)))
  ;[1 1 1] Rush
  (if (not (`self.IsUsingRush`))
    (set `self.IsUsingRush` true)
    (bind _outhit (`KismetSystemLibrary.LineTraceSingle` :`Start` _returnvalue :`End` (+ _returnvalue (* (+ (`SceneComponent.GetForwardVector` _firstpersoncamera) (`KismetMathLibrary.Conv_RotatorToVector` (`SceneComponent.K2_GetComponentRotation` _firstpersoncamera))) 200.0)) :`TraceChannel` "TraceTypeQuery1" :`DrawDebugType` "Persistent"))
    (bind (_bblockinghit _binitialoverlap _time _distance _location _impactpoint _normal _impactnormal _physmat _hitactor _hitcomponent _hitbonename _hititem _elementindex _faceindex _tracestart _traceend) (`GameplayStatics.BreakHitResult` _outhit))
    (if _bblockinghit
      (bind _outhit_2 (`KismetSystemLibrary.LineTraceSingle` _impactpoint (- _impactpoint (0.0 0.0 150.0)) "TraceTypeQuery1"))
      (if (`GameplayStatics.BreakHitResult` _outhit_2)
        (`self.K2_SetActorLocation` (- _impactpoint (- (`self.GetActorForwardVector`) (100.0 0.0 0.0))) true))
      (set `self.IsUsingRush` false)
      (else
        (bind _outhit_3 (`KismetSystemLibrary.LineTraceSingle` :`Start` _traceend :`End` (- _traceend (0.0 0.0 150.0)) :`TraceChannel` "TraceTypeQuery1" :`DrawDebugType` "Persistent"))
        (if (`GameplayStatics.BreakHitResult` _outhit_3)
          (`self.K2_SetActorLocation` _traceend true))
        (set `self.IsUsingRush` false)))))

(event `Key|A`
  (params (Key :type "Key Structure"))
  ;[1 1 1] ThrowingKnife Skill logic
  (:`Pressed`
    (`self.DaggerThrow` (`SceneComponent.K2_GetComponentRotation` (`self.FirstPersonCamera`)))))

(event `DaggerThrow`
  (params (`z rotator` :type "Rotator Structure"))
  ;[1 1 1] ThrowingKnife Skill logic
  (if (not (`self.IsThrowingDagger`))
    (set `self.IsThrowingDagger` true)
    (`|SpawnActorFromClass` "/Game/_Game/_Core/Weapons/Physical_competence/DaggerThrow/BP_DaggerThrow.BP_DaggerThrow_C" (`KismetMathLibrary.MakeTransform` (`SceneComponent.K2_GetComponentLocation` (`self.SpawnMeleeDegat`)) `z rotator`) "Undefined" "OverrideRootScale" null null)
    (`KismetSystemLibrary.Delay` 1.0)
    (set `self.IsThrowingDagger` false)))

(event `Key|E`
  (params (Key :type "Key Structure"))
  ;[1 1 1] Débarquement logic
  (:`Pressed`
    (`self.Débarquement` (`SceneComponent.K2_GetComponentRotation` (`self.FirstPersonCamera`)))))

(event `Débarquement`
  (params (`Z AXIS` :type "Rotator Structure"))
  ;[1 1 1] Débarquement logic
  (if (not (`self.IsUsingCrush`))
    (set `self.IsUsingCrush` true)
    (`|SpawnActorFromClass` "/Game/_Game/_Core/Weapons/Physical_competence/Debarquement/BP_Crush.BP_Crush_C" (`KismetMathLibrary.MakeTransform` (`SceneComponent.K2_GetComponentLocation` (`self.SpawnCrush`))) "AlwaysSpawn" "OverrideRootScale" null null)
    (set `self.IsUsingCrush` false)))

(fn `UserConstructionScript`
  (`parent.UserConstructionScript`))