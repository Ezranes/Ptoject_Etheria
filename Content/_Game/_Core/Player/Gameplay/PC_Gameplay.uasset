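; PC_Gameplay is the gameplay player controller that sets up the main gameplay HUD and relays character spawn requests.
; On BeginPlay, the local controller creates WBP_MainGameplay, adds it to the viewport, and caches it along with the MainGameInstance.
; Its SpawnCharacterOnGameMode event casts the game mode to GM_Gameplay and forwards the given character and controller to its SpawnCharacter function.
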(event `self.ReceiveBeginPlay`
  (if (`self.IsLocalController`)
    (`|ExecutionSequence`
      (:`then_0`
        (bind _returnvalue (`|CreateWidget` "/Game/_Game/UI/MainGame/Pages/WBP_MainGameplay.WBP_MainGameplay_C" self))
        (`UserWidget.AddToViewport` _returnvalue 0)
        (set `self.WBP_MainGameplay` _returnvalue))
      (:`then_1`
        (bind _asmain_game_instance (cast `/Game/_Game/_Core/Framework/General/MainGameInstance` (`GameplayStatics.GetGameInstance`)))
        (set `self.GameInstance` _asmain_game_instance)))))

(event `SpawnCharacterOnGameMode`
  (params (Character :type "Character Class Reference") (controller :type "Controller Object Reference"))
  (bind _asgm_gameplay (cast `/Game/_Game/_Core/Framework/Gameplay/GM_Gameplay` (`GameplayStatics.GetGameMode`)))
  (`/Game/_Game/_Core/Framework/Gameplay/GM_Gameplay.SpawnCharacter` _asgm_gameplay Character controller))

(fn `UserConstructionScript`)