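; BP_Crush is a player skill actor that creates a scaling area effect which stuns _Mother actors it touches.
; On BeginPlay, the Crush timeline scales both Sphere and Detector from the actor's initial relative scale to VectorEND.
; Detector overlaps add each _Mother to ActorTouched and call Stuning on it with that whole array and a true stun flag.
; Leaving the Detector only removes the actor from the array, with no un-stun call.
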(event `self.ReceiveBeginPlay`
  (set `self.VectorScale` (`self.GetActorRelativeScale3D`))
  (bind (_direction _crush) (`Timeline|Crush` :!via `PlayFromStart`)
    (:`Update`
      (bind _returnvalue (`KismetMathLibrary.VLerp` (`self.VectorScale`) (`self.VectorEND`) _crush))
      (`SceneComponent.SetRelativeScale3D` (`self.Sphere`) _returnvalue)
      (`SceneComponent.SetRelativeScale3D` (`self.Detector`) _returnvalue))))

(event `self.Detector.OnComponentBeginOverlap`
  (params (OverlappedComponent :type "PrimitiveComponent Object Reference") (OtherActor :type "Actor Object Reference") (OtherComp :type "PrimitiveComponent Object Reference") (OtherBodyIndex :type Integer) (bFromSweep :type Boolean) (SweepResult :type "HitResult Structure (by ref)"))
  (bind _actor_touched (`self.Actor touched`))
  (bind _as_mother (cast `/Game/_CORE/Player/IA/_Mother` OtherActor))
  (`KismetArrayLibrary.Array_AddUnique` _actor_touched _as_mother)
  (bind _output_get (set `self.stuned ?` true))
  (`/Game/_CORE/Player/IA/_Mother.stuning` _as_mother _actor_touched _output_get))

(event `self.Detector.OnComponentEndOverlap`
  (params (OverlappedComponent :type "PrimitiveComponent Object Reference") (OtherActor :type "Actor Object Reference") (OtherComp :type "PrimitiveComponent Object Reference") (OtherBodyIndex :type Integer))
  (bind _as_mother (cast `/Game/_CORE/Player/IA/_Mother` OtherActor))
  (`KismetArrayLibrary.Array_RemoveItem` (`self.Actor touched`) _as_mother))

(fn `UserConstructionScript`)