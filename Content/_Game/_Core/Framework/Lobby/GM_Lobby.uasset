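; GM_Lobby is the lobby game mode that tracks connected players and starts level travel for the session.
; On login it adds the PC_Lobby controller to PlayerList, waits briefly, then pushes the list to every controller's valid lobby widget.
; Logout only removes the controller from the list, without refreshing the widgets.
; ServerTravel runs a servertravel console command built from the given level name.
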(event `self.ReceiveBeginPlay`)

(event `self.K2_PostLogin`
  (params (NewPlayer :type "PlayerController Object Reference"))
  (bind _playerlist (`self.PlayerList`))
  (bind _aspc_lobby (cast `/Game/_Game/_Core/Player/Lobby/PC_Lobby` NewPlayer))
  (`KismetArrayLibrary.Array_Add` _playerlist _aspc_lobby)
  (`KismetSystemLibrary.Delay` 0.2)
  (for _array_element _playerlist
    (bind _wbplobby (`/Game/_Game/_Core/Player/Lobby/PC_Lobby.WBPLobby` _array_element))
    (`/Engine/EditorBlueprintResources/StandardMacros.IsValid` _wbplobby
      (:`Is Valid`
        (`/Game/_Game/UI/MainMenu/Pages/WBP_Lobby.UpdateListPlayers` _wbplobby _playerlist)))))

(event `self.K2_OnLogout`
  (params (ExitingController :type "Controller Object Reference"))
  (bind _aspc_lobby (cast `/Game/_Game/_Core/Player/Lobby/PC_Lobby` ExitingController))
  (`KismetArrayLibrary.Array_RemoveItem` (`self.PlayerList`) _aspc_lobby))

(event `ServerTravel`
  (params (levelName :type String))
  (`KismetSystemLibrary.ExecuteConsoleCommand` (`KismetStringLibrary.Concat_StrStr` "servertravel " levelName) null))

(fn `UserConstructionScript`)