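; PC_Menu is the main menu player controller, linking the menu UI to multiplayer session hosting, searching and joining.
; On BeginPlay it creates WBP_MainMenu, then caches MainGameInstance after a one-second delay.
; Client events forward session requests and player registration to that GameInstance, showing a throbber while searching or joining.
; It also builds server and player entry widgets; UpdatePlayerListLobby only delays, and M prints the player count.
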(event `self.ReceiveBeginPlay`
  ;[1 1 1] BeginPlay
  (`self.CreateMainMenus`)
  (`KismetSystemLibrary.Delay` 1.0)
  (`self.Getting gameInstance`))

(event `Getting gameInstance`
  ;[1 1 1] gameinstance references
  (bind _asmain_game_instance (cast `/Game/_Game/_Core/Framework/General/MainGameInstance` (`GameplayStatics.GetGameInstance`)))
  (set `self.GameInstance` _asmain_game_instance))

(event `CreateMainMenus`
  ;[1 1 1] create menus on screen
  (bind _returnvalue (`|CreateWidget` "/Game/_Game/UI/MainMenu/Pages/WBP_MainMenu.WBP_MainMenu_C" (`GameplayStatics.GetPlayerController` 0)))
  (bind _output_get (set `self.WBP_MainMenu` _returnvalue))
  (`UserWidget.AddToViewport` _output_get 0))

(event `ClientWantToHost`
  (params (servername :type String))
  ;[1 1 1] Host server
  (`/Game/_Game/_Core/Framework/General/MainGameInstance.HostSession` (`self.GameInstance`) self servername))

(event `ClientFindSession`
  ;[1 1 1] Searching game
  (`/Game/_Game/UI/MainMenu/Pages/WBP_MainMenu.Activate Throbber` (`self.WBP_MainMenu`) "searching Session...")
  (`/Game/_Game/_Core/Framework/General/MainGameInstance.FindSessions` (`self.GameInstance`) self))

(event `CreateServerEntries`
  (params (TargetsServer :type "BlueprintSessionResult Structure"))
  ;[1 1 1] create servers entries
  (bind _returnvalue (`|CreateWidget` "/Game/_Game/UI/MainMenu/Partials/ServerList/WBP_ServerEntry.WBP_ServerEntry_C" null TargetsServer))
  (`PanelWidget.AddChild` (`/Game/_Game/UI/MainMenu/Pages/WBP_MainMenu.ServerContainerBox` (`self.WBP_MainMenu`)) _returnvalue)
  (`KismetArrayLibrary.Array_Add` (`self.ServerList`) _returnvalue))

(event `Register player`
  ;[1 0 0] Comment
  ;;[1 1 1] Register player
  (`/Game/_Game/_Core/Framework/General/MainGameInstance.PlayerJoined` (`self.GameInstance`) self))

(event `Key|M`
  (params (Key :type "Key Structure"))
  ;[1 0 0] Comment
  (:`Pressed`
    (`self.Server test`)))

(event `Server test`
  ;[1 0 0] Comment
  (`KismetSystemLibrary.PrintString` (`KismetStringLibrary.Conv_IntToString` (`/Game/_Game/_Core/Framework/General/MainGameInstance.NumberOfPlayer` (`self.GameInstance`)))))

(event `Client Disable Throbber`
  ;[1 0 0] Comment
  ;;[1 1 1] disable Throbber
  (`/Game/_Game/UI/MainMenu/Pages/WBP_MainMenu.DisableThrobber` (`self.WBP_MainMenu`)))

(event `CreateSessiongame`
  ;[1 0 0] Comment
  (bind _aspc_menu (cast `/Game/_Game/_Core/Player/Menu/PC_Menu` (`GameplayStatics.GetPlayerController` 0)))
  (`/Game/_Game/_Core/Framework/General/MainGameInstance.HostSession` (`/Game/_Game/_Core/Player/Menu/PC_Menu.GameInstance` _aspc_menu) null ""))

(event `RemoveServerEntries`
  ;[1 0 0] Comment
  ;;[1 1 1] Remove server Entries
  (for _array_element (`self.ServerList`)
    (`Widget.RemoveFromParent` _array_element)))

(event `JoinSessionGame`
  ;[1 0 0] Comment
  (bind _aspc_menu (cast `/Game/_Game/_Core/Player/Menu/PC_Menu` (`GameplayStatics.GetPlayerController` 0)))
  (`/Game/_Game/_Core/Framework/General/MainGameInstance.JoinSession` :`self` (`/Game/_Game/_Core/Player/Menu/PC_Menu.GameInstance` _aspc_menu)))

(event `ClientJoinSession`
  (params (TargetSession :type "BlueprintSessionResult Structure"))
  ;[1 0 0] Comment
  ;;[1 1 1] joining Logic
  (`/Game/_Game/UI/MainMenu/Pages/WBP_MainMenu.Activate Throbber` (`self.WBP_MainMenu`) "Joining...")
  (`/Game/_Game/_Core/Framework/General/MainGameInstance.JoinSession` (`self.GameInstance`) self TargetSession))

(event `Create Player Entries`
  (params (TargetsServer :type "/Game/_Game/_Core/Player/Lobby/PS_Lobby Object Reference"))
  ;[1 0 0] Comment
  ;;[1 1 1] create Player entries
  (bind _returnvalue (`|CreateWidget` "/Game/_Game/UI/MainMenu/_BACKUP/UI_OUT_iTryAgain/WBP_PlayerEntrie.WBP_PlayerEntrie_C"))
  (`/Engine/EditorBlueprintResources/StandardMacros.IsValid` _returnvalue
    (:`Is Valid`
      (`PanelWidget.AddChild` (`/Game/_Game/UI/MainMenu/_BACKUP/UI_OUT_iTryAgain/WBP_Menus.PlayerEntriesBox_1` (`self.As PC_menus`)) _returnvalue)
      (`KismetArrayLibrary.Array_Add` (`self.PlayerList`) _returnvalue))))

(event `UpdatePlayerListLobby`
  (params (ListPlayers :type "Array of /Game/_Game/_Core/Player/Menu/PC_Menu Object Reference"))
  ;[1 0 0] Comment
  (`KismetSystemLibrary.Delay` 0.2))

(fn `UserConstructionScript`)