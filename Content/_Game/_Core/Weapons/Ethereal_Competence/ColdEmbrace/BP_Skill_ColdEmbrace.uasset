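; BP_Skill_ColdEmbrace is the Cold Embrace skill actor, an area damage effect that hurts _Mother actors inside its sphere.
; Sphere overlap begin and end events add and remove those actors in a tracked array without duplicates.
; Tick applies fixed damage to every tracked actor each frame with itself as causer, unscaled by delta time, so damage rate follows frame rate.
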(event `self.ReceiveTick`
  (params (DeltaSeconds :type "Float (single-precision)"))
  (for _array_element (`self.As _Mother`)
    (`GameplayStatics.ApplyDamage` _array_element 100.0 null self)))

(event `self.Sphere.OnComponentBeginOverlap`
  (params (OverlappedComponent :type "PrimitiveComponent Object Reference") (OtherActor :type "Actor Object Reference") (OtherComp :type "PrimitiveComponent Object Reference") (OtherBodyIndex :type Integer) (bFromSweep :type Boolean) (SweepResult :type "HitResult Structure (by ref)"))
  (bind _as_mother (cast `/Game/_Game/_Core/IA/_Mother` OtherActor))
  (`KismetArrayLibrary.Array_AddUnique` (`self.As _Mother`) _as_mother))

(event `self.Sphere.OnComponentEndOverlap`
  (params (OverlappedComponent :type "PrimitiveComponent Object Reference") (OtherActor :type "Actor Object Reference") (OtherComp :type "PrimitiveComponent Object Reference") (OtherBodyIndex :type Integer))
  (bind _as_mother (cast `/Game/_Game/_Core/IA/_Mother` OtherActor))
  (`KismetArrayLibrary.Array_RemoveItem` (`self.As _Mother`) _as_mother))

(fn `UserConstructionScript`)