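; Playable Ethereal character with a primary Spirit Shot and three abilities: Cold Embrace, Lightning and a Shadow Run blink.
; Input keys call ability events, each guarded by a busy flag, with short delays as cooldowns on spawned abilities.
; Camera-directed line traces place Cold Embrace, restrict Lightning to _Mother actors and set the Shadow Run destination.
; BeginPlay initializes health (Vie); the health and mana bar functions are empty.
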(event `Key|LeftMouseButton`
  (params (Key :type "Key Structure"))
  ;[1 1 1] Logique du tir du spirit shot
  (:`Pressed`
    (`self.ShootingButton` (`SceneComponent.K2_GetComponentRotation` (`self.Sphere`)))))

(event `ShootingButton`
  (params (Rotator :type "Rotator Structure"))
  ;[1 1 1] Logique du tir du spirit shot
  (if (not (`self.Shooting`))
    (set `self.Shooting` true)
    (`|SpawnActorFromClass` "/Game/_Game/_Core/Weapons/Spirit_Shot/Spirit_Shot.Spirit_Shot_C" (`KismetMathLibrary.MakeTransform` (`SceneComponent.K2_GetComponentLocation` (`self.Sphere`)) Rotator) "AlwaysSpawn" "OverrideRootScale" self null)
    (`KismetSystemLibrary.Delay` 0.5)
    (set `self.Shooting` false)))

(event `Key|A`
  (params (Key :type "Key Structure"))
  ;[1 1 1] Logique de spawn du skill ColdEmbrace
  (:`Pressed`
    (`self.ColdEmbrace` (`SceneComponent.K2_GetComponentRotation` (`self.FirstPersonCamera`)))))

(event `ColdEmbrace`
  (params (`z rotation` :type "Rotator Structure"))
  (bind _returnvalue (`SceneComponent.K2_GetComponentLocation` (`self.Sphere`)))
  ;[1 1 1] Logique de spawn du skill ColdEmbrace
  (if (not (`self.IsUsingSkill1`))
    (set `self.IsUsingSkill1` true)
    (bind (_outhit _returnvalue_2) (`KismetSystemLibrary.LineTraceSingle` _returnvalue (+ _returnvalue (* (+ (`SceneComponent.GetForwardVector` (`self.FirstPersonCamera`)) (`KismetMathLibrary.Conv_RotatorToVector` `z rotation`)) 500.0)) "TraceTypeQuery1"))
    (if _returnvalue_2
      (`|SpawnActorFromClass` "/Game/_Game/_Core/Weapons/Ethereal_Competence/ColdEmbrace/BP_Skill_ColdEmbrace.BP_Skill_ColdEmbrace_C" (`KismetMathLibrary.MakeTransform` (`.ImpactPoint` (`GameplayStatics.BreakHitResult` _outhit))) "AlwaysSpawn" "OverrideRootScale" null null)
      (`KismetSystemLibrary.Delay` 1.0))
    (set `self.IsUsingSkill1` false)))

(event `Key|E`
  (params (Key :type "Key Structure"))
  ;[1 1 1] Logique de spawn du Lightning
  (:`Pressed`
    (`self.Lightning`)))

(event `Lightning`
  (bind _returnvalue (`SceneComponent.K2_GetComponentLocation` (`self.Sphere`)))
  ;[1 1 1] Logique de spawn du Lightning
  (if (not (`self.IsUsingSkill2`))
    (set `self.IsUsingSkill2` true)
    (bind _outhit (`KismetSystemLibrary.LineTraceSingle` :`Start` _returnvalue :`End` (+ _returnvalue (* (+ (`SceneComponent.GetForwardVector` (`self.FirstPersonCamera`)) (`KismetMathLibrary.Conv_RotatorToVector` (`SceneComponent.K2_GetComponentRotation` (`self.FirstPersonCamera`)))) 250.0)) :`TraceChannel` "TraceTypeQuery1" :`DrawDebugType` "Persistent"))
    (bind (_bblockinghit _binitialoverlap _time _distance _location _impactpoint _normal _impactnormal _physmat _hitactor) (`GameplayStatics.BreakHitResult` _outhit))
    (cast `/Game/_Game/_Core/IA/_Mother` _hitactor
      (:`then`
        (`|SpawnActorFromClass` "/Game/_Game/_Core/Weapons/Ethereal_Competence/Lightning/Lightning.Lightning_C" (`KismetMathLibrary.MakeTransform` (`self.K2_GetActorLocation` _hitactor)) "AlwaysSpawn" "OverrideRootScale" null null)
        (`|SpawnActorFromClass` "/Game/_Game/_Core/Weapons/Ethereal_Competence/Lightning/BP_TP_LightningFX.BP_TP_LightningFX_C" (`KismetMathLibrary.MakeTransform` (`self.K2_GetActorLocation` self)) "Undefined" "OverrideRootScale" self null)
        (`KismetSystemLibrary.Delay` 1.0))
      (:`CastFailed`
        _))
    (set `self.IsUsingSkill2` false)))

(event `Key|R`
  (params (Key :type "Key Structure"))
  ;[1 1 1] Shadow Run logique
  (:`Pressed`
    (`self.ShadowRunActivation` (`SceneComponent.K2_GetComponentRotation` (`self.FirstPersonCamera`)))))

(event `ShadowRunActivation`
  (params (`z axis` :type "Rotator Structure"))
  (bind _returnvalue (`SceneComponent.K2_GetComponentLocation` (`self.Sphere`)))
  ;[1 1 1] Shadow Run logique
  (if (not (`self.Is shadow running`))
    (set `self.Is shadow running` true)
    (bind _outhit (`KismetSystemLibrary.LineTraceSingle` :`Start` _returnvalue :`End` (+ _returnvalue (* (+ (`SceneComponent.GetForwardVector` (`self.FirstPersonCamera`)) (`KismetMathLibrary.Conv_RotatorToVector` `z axis`)) 150.0)) :`TraceChannel` "TraceTypeQuery1" :`DrawDebugType` "Persistent"))
    (bind (_bblockinghit _binitialoverlap _time _distance _location _impactpoint _normal _impactnormal _physmat _hitactor _hitcomponent _hitbonename _hititem _elementindex _faceindex _tracestart _traceend) (`GameplayStatics.BreakHitResult` _outhit))
    (if _bblockinghit
      (`self.K2_SetActorLocation` (- _impactpoint (- (`SceneComponent.GetForwardVector` (`self.FirstPersonCamera`)) (-100.0 0.0 0.0))) false true)
      (else
        (`self.K2_SetActorLocation` _traceend)))
    (set `self.Is shadow running` false)))

(event `self.ReceiveBeginPlay`
  (set `self.Vie` 100.0))

(fn `HealthBarFunction`)

(fn `ManaBarFunction`)

(fn `UserConstructionScript`
  (`parent.UserConstructionScript`))